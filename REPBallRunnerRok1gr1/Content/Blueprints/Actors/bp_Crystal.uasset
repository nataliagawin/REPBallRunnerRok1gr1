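; A crystal actor that flies to the player and vanishes when the player overlaps its sphere.
; On overlap it caches its location, scale and point light intensity, then plays a timeline.
; The timeline lerps it toward the player pawn's current location, re-read each update, while shrinking it and fading its light to zero, then destroys the actor.
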(event OnComponentBeginOverlap(Sphere)
  (params (OverlappedComponent :type Primitive%20Component%20Object%20Reference) (OtherActor :type Actor%20Object%20Reference) (OtherComp :type Primitive%20Component%20Object%20Reference) (OtherBodyIndex :type Integer) (bFromSweep :type Boolean) (SweepResult :type Hit%20Result%20Structure%20%28by%20ref%29))
  (Utilities|IsPlayer OtherActor
    (:True
      (CallFunction|SetProperties)
      (bind (_direction _lerpmovement _lerpscale _lerplight) (Timeline|CrystalTimeMovement Play)
        (:Update
          (CallFunction|LerpLocation _lerpmovement)
          (CallFunction|LerpScale _lerpscale)
          (CallFunction|LerpLight _lerplight))
        (:Finished
          (Actor|DestroyActor))))))

(fn ConstructionScript)

(fn LerpLight
  (params (Alpha :type Float%20%28single-precision%29))
  (Rendering|Components|Light|SetIntensity (Variables|Default|GetPointLight) (Math|Float|Lerp (Variables|CrystalProperties|GetCrystalIntensity) 0.0 Alpha)))

(fn LerpScale
  (params (Alpha :type Float%20%28single-precision%29))
  (Transformation|SetActorScale3D (Math|Vector|Lerp(Vector) (Variables|CrystalProperties|GetCrystalScale) "0, 0, 0" Alpha)))

(fn LerpLocation
  (params (Alpha :type Float%20%28single-precision%29))
  (Transformation|SetActorLocation (Math|Vector|Lerp(Vector) (Variables|CrystalProperties|GetCrystalLocation) (Transformation|GetActorLocation (Game|Player|GetPlayerPawn 0)) Alpha) false false))

(fn SetProperties
  (Variables|CrystalProperties|SetCrystalLocation (Transformation|GetActorLocation))
  (Variables|CrystalProperties|SetCrystalScale (Transformation|GetActorScale3D))
  (Variables|CrystalProperties|SetCrystalIntensity (Variables|/Script/Engine.LightComponentBase|GetIntensity (Variables|Default|GetPointLight))))